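; Player controller that steers its controlled pawn continuously toward the world point under the mouse cursor.
; Every tick, a complex Visibility trace under the cursor supplies a target, and the normalized direction from the pawn to that point feeds Add Movement Input at full scale.
; Disconnected nodes for hiding the cursor and rotating the pawn toward the target with a pitch offset never run.
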(event EventTick
  (params (DeltaSeconds :type Float%20%28single-precision%29))
  (bind _returnvalue (Pawn|GetControlledPawn))
  (Pawn|Input|AddMovementInput _returnvalue (Math|Vector|Normalize (Math|Vector|GetUnitDirection(Vector) (Transformation|GetActorLocation _returnvalue) (.Location (Collision|BreakHitResult (.HitResult (Game|Player|GetHitResultUnderCursorbyChannel "TraceTypeQuery1" true)))))) 1.0 false))

(event Input|ActionEvents|InputActionToggleMovement
  (params (Key :type Key%20Structure :default "None")))

(fn ConstructionScript)